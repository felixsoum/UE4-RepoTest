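; BP_Enemy is an enemy that endlessly alternates slash and throw attack montages aimed at the player.
; BeginPlay runs a loop that waits a second, faces the player, plays a montage, and starts the next step when that montage completes.
; The FacePlayer function snaps the actor's rotation toward player pawn 0 on the horizontal plane, flattening Z so it stays upright.
; Montage interruption is unhandled, so an interrupted attack stops the loop.
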(event `self.ReceiveBeginPlay`
  (`KismetSystemLibrary.Delay` 1.0 :!label _label)
  (`self.FacePlayer`
    (:`Out`
      (`|PlayMontage` (`self.Mesh`) "/Game/Enemy/AM_Slash.AM_Slash"
        (:`OnCompleted`
          (`KismetSystemLibrary.Delay` 1.0)
          (`self.FacePlayer`
            (:`Out`
              (`|PlayMontage` (`self.Mesh`) "/Game/Enemy/AM_Throw.AM_Throw"
                (:`OnCompleted`
                  (goto _label))))))))))

(fn `UserConstructionScript`)